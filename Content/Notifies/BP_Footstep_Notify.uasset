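; Animation notify that plays surface-specific footstep sounds.
; GetSurface line-traces 150 units down from player character 0, not the animated mesh's owner, on the Visibility channel.
; It switches on the hit's physical surface to play a sound at the impact and return an index, with Dirt sound as default.
; Received_Notify stores that index, but its checks on it only return true.
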(fn ReceivedNotify
  (params (MeshComp :type Skeletal%20Mesh%20Component%20Object%20Reference) (Animation :type Anim%20Sequence%20Base%20Object%20Reference) (EventReference :type Anim%20Notify%20Event%20Reference%20Structure%20%28by%20ref%29))
  (Utilities|IsValid MeshComp
    (:Is%20Valid
      (bind _surface (CallFunction|GetSurface))
      (bind _output_get (LocalVariables|SetSurfaceType _surface))
      (Utilities|FlowControl|Sequence
        (:then_0
          (if (== _output_get 0)
            (return true)))
        (:then_1
          (if (== _output_get 1)
            (return true)))))
    (:Is%20Not%20Valid
      (return true))))

(fn GetSurface
  (bind _returnvalue (Game|GetPlayerCharacter 0))
  (bind _returnvalue_2 (Transformation|GetActorLocation _returnvalue))
  (bind (_outhit _returnvalue_3) (Collision|LineTraceByChannel _returnvalue_2 (- _returnvalue_2 "0.000000,0.000000,150.000000") "TraceTypeQuery1" false 0 "None"))
  (if _returnvalue_3
    (switch Utilities|FlowControl|Switch|SwitchonEPhysicalSurface (Collision|GetSurfaceType _outhit)
      (:SurfaceType_Default
        (LocalVariables|SetSurfaceTypeNum 0)
        (Audio|PlaySoundatLocation "/Game/Audio/Footstep_Sounds_Pro/Dirt_footsteps/SQ_Footsteps_Dirt.SQ_Footsteps_Dirt" (.Location (Collision|BreakHitResult _outhit)) "0, 0, 0" 1.0 1.0 0.0 0 0 0 0)
        (return (LocalVariables|GetSurfaceTypeNum)))
      (:SurfaceType1
        (LocalVariables|SetSurfaceTypeNum 1)
        (Audio|PlaySoundatLocation "/Game/Audio/Footstep_Sounds_Pro/Concrete_footsteps/SQ_Footsteps_Concrete.SQ_Footsteps_Concrete" (.Location (Collision|BreakHitResult _outhit)) "0, 0, 0" 1.0 1.0 0.0 0 0 0 0)
        (return (LocalVariables|GetSurfaceTypeNum)))
      (:SurfaceType2
        (LocalVariables|SetSurfaceTypeNum 2)
        (Audio|PlaySoundatLocation "/Game/Audio/Footstep_Sounds_Pro/Dirt_footsteps/SQ_Footsteps_Dirt.SQ_Footsteps_Dirt" (.Location (Collision|BreakHitResult _outhit)) "0, 0, 0" 1.0 1.0 0.0 0 0 0 0)
        (return (LocalVariables|GetSurfaceTypeNum)))
      (:SurfaceType3
        (LocalVariables|SetSurfaceTypeNum 3)
        (Audio|PlaySoundatLocation "/Game/Audio/Footstep_Sounds_Pro/Glass_footsteps/SQ_Footsteps_Glass.SQ_Footsteps_Glass" (.Location (Collision|BreakHitResult _outhit)) "0, 0, 0" 1.0 1.0 0.0 0 0 0 0)
        (return (LocalVariables|GetSurfaceTypeNum)))
      (:SurfaceType4
        (LocalVariables|SetSurfaceTypeNum 4)
        (Audio|PlaySoundatLocation "/Game/Audio/Footstep_Sounds_Pro/Grass_footsteps/SQ_Footsteps_Grass.SQ_Footsteps_Grass" (.Location (Collision|BreakHitResult _outhit)) "0, 0, 0" 1.0 1.0 0.0 0 0 0 0)
        (return (LocalVariables|GetSurfaceTypeNum)))
      (:SurfaceType5
        (LocalVariables|SetSurfaceTypeNum 5)
        (Audio|PlaySoundatLocation "/Game/Audio/Footstep_Sounds_Pro/Gravel_Footsteps/SQ_Footstaps_Gravel.SQ_Footstaps_Gravel" (.Location (Collision|BreakHitResult _outhit)) "0, 0, 0" 1.0 1.0 0.0 0 0 0 0)
        (return (LocalVariables|GetSurfaceTypeNum)))
      (:SurfaceType6
        (LocalVariables|SetSurfaceTypeNum 6)
        (Audio|PlaySoundatLocation "/Game/Audio/Footstep_Sounds_Pro/Ice_Footsteps/SQ_Footsteps_Ice.SQ_Footsteps_Ice" (.Location (Collision|BreakHitResult _outhit)) "0, 0, 0" 1.0 1.0 0.0 0 0 0 0))
      (:SurfaceType7
        (LocalVariables|SetSurfaceTypeNum 7)
        (Audio|PlaySoundatLocation "/Game/Audio/Footstep_Sounds_Pro/Metal_footsteps/SQ_Footsteps_Metal.SQ_Footsteps_Metal" (.Location (Collision|BreakHitResult _outhit)) "0, 0, 0" 1.0 1.0 0.0 0 0 0 0)
        (return (LocalVariables|GetSurfaceTypeNum)))
      (:SurfaceType8
        (LocalVariables|SetSurfaceTypeNum 8)
        (Audio|PlaySoundatLocation "/Game/Audio/Footstep_Sounds_Pro/Mud_footsteps/SQ_Footsteps_Mud.SQ_Footsteps_Mud" (.Location (Collision|BreakHitResult _outhit)) "0, 0, 0" 1.0 1.0 0.0 0 0 0 0)
        (return (LocalVariables|GetSurfaceTypeNum)))
      (:SurfaceType9
        (LocalVariables|SetSurfaceTypeNum 9)
        (Audio|PlaySoundatLocation "/Game/Audio/Footstep_Sounds_Pro/Sand_footsteps/SQ_Footsteps_Sand.SQ_Footsteps_Sand" (.Location (Collision|BreakHitResult _outhit)) "0, 0, 0" 1.0 1.0 0.0 0 0 0 0)
        (return (LocalVariables|GetSurfaceTypeNum)))
      (:SurfaceType10
        (LocalVariables|SetSurfaceTypeNum 10)
        (Audio|PlaySoundatLocation "/Game/Audio/Footstep_Sounds_Pro/Snow_footsteps/SQ_Footsteps_Snow.SQ_Footsteps_Snow" (.Location (Collision|BreakHitResult _outhit)) "0, 0, 0" 1.0 1.0 0.0 0 0 0 0)
        (return (LocalVariables|GetSurfaceTypeNum)))
      (:SurfaceType11
        (LocalVariables|SetSurfaceTypeNum 11)
        (Audio|PlaySoundatLocation "/Game/Audio/Footstep_Sounds_Pro/Stone_footsteps/SQ_Footsteps_Stone.SQ_Footsteps_Stone" (.Location (Collision|BreakHitResult _outhit)) "0, 0, 0" 1.0 1.0 0.0 0 0 0 0)
        (return (LocalVariables|GetSurfaceTypeNum)))
      (:SurfaceType12
        (LocalVariables|SetSurfaceTypeNum 12)
        (Audio|PlaySoundatLocation "/Game/Audio/Footstep_Sounds_Pro/Water_footsteps/SQ_Footsteps_Water.SQ_Footsteps_Water" (.Location (Collision|BreakHitResult _outhit)) "0, 0, 0" 1.0 1.0 0.0 0 0 0 0)
        (return (LocalVariables|GetSurfaceTypeNum)))
      (:SurfaceType13
        (LocalVariables|SetSurfaceTypeNum 13)
        (Audio|PlaySoundatLocation "/Game/Audio/Footstep_Sounds_Pro/Wood_footsteps/SQ_Footsteps_Wood.SQ_Footsteps_Wood" (.Location (Collision|BreakHitResult _outhit)) "0, 0, 0" 1.0 1.0 0.0 0 0 0 0)
        (return (LocalVariables|GetSurfaceTypeNum))))))