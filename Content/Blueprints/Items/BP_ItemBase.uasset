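; Base item actor that shows proximity interaction icons and can be interacted with by the first-person character.
; A far collision volume shows the far icon while the player character overlaps it, hiding both icons on exit.
; The CanInteract event toggles the near icon without changing the far one.
; Interact destroys the item only if it is the interacting character's CurrentHitInteractable.
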(event OnComponentBeginOverlap(FarCollision)
  (params (OverlappedComponent :type Primitive%20Component%20Object%20Reference) (OtherActor :type Actor%20Object%20Reference) (OtherComp :type Primitive%20Component%20Object%20Reference) (OtherBodyIndex :type Integer) (bFromSweep :type Boolean) (SweepResult :type Hit%20Result%20Structure%20%28by%20ref%29))
  ;[0.15 0.15 0.15 0.5] Far Collision Trigger
  (if (== OtherActor (Game|GetPlayerCharacter 0))
    (Rendering|SetVisibility (Variables|Default|GetFarInteractIcon) true false)
    (Rendering|SetVisibility (Variables|Default|GetNearInteractIcon) false false)))

(event OnComponentEndOverlap(FarCollision)
  (params (OverlappedComponent :type Primitive%20Component%20Object%20Reference) (OtherActor :type Actor%20Object%20Reference) (OtherComp :type Primitive%20Component%20Object%20Reference) (OtherBodyIndex :type Integer))
  ;[0.15 0.15 0.15 0.5] Far Collision Trigger
  (if (== (Game|GetPlayerCharacter 0) OtherActor)
    (Rendering|SetVisibility (Variables|Default|GetFarInteractIcon) false false)
    (Rendering|SetVisibility (Variables|Default|GetNearInteractIcon) false false)))

(event EventBeginPlay
  (Rendering|SetVisibility (Variables|Default|GetNearInteractIcon) false false)
  (Rendering|SetVisibility (Variables|Default|GetFarInteractIcon) false false))

(event EventInteract
  (params (Interactor :type Character%20Object%20Reference))
  (bind _asbp_first_person_character (Utilities|Casting|CastToBP_FirstPersonCharacter Interactor))
  (if (== (Variables|/Game/Blueprints/GameFramework/BP_FirstPersonCharacter.BP_FirstPersonCharacter_C|GetCurrentHitInteractable _asbp_first_person_character) self)
    (Actor|DestroyActor)))

(event EventCanInteract
  (params (bCanInteract :type Boolean))
  (Rendering|SetVisibility (Variables|Default|GetNearInteractIcon) bCanInteract false))

(fn ConstructionScript)