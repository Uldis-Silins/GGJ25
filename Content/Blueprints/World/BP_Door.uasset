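; Interactable door that cycles through closed, partially open and open, with a sound for each transition and near/far prompt icons.
; Interacting picks the swing side from a dot product of player and door facing, then Tick interpolates the yaw until a timer advances the state.
; Optional auto-close forces the closing transition when the player leaves the box, while sphere overlap and the interface's CanInteract toggle the icons.
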(event OnComponentEndOverlap(Box)
  (params (OverlappedComponent :type Primitive%20Component%20Object%20Reference) (OtherActor :type Actor%20Object%20Reference) (OtherComp :type Primitive%20Component%20Object%20Reference) (OtherBodyIndex :type Integer))
  ;[0.15 0.15 0.15 0.5] Auto Close
  (if (or (Utilities|Enum|NotEqual(Enum) (Variables|Default|GetCurrentDoorState) "NewEnumerator0") (Variables|Default|GetbIsInteracting))
    (if (and (Variables|Door|GetbAutoClose) (== OtherActor (Game|GetPlayerCharacter 0)))
      (Variables|Default|SetCurrentDoorState "NewEnumerator2")
      (bind _asbp_first_person_character (Utilities|Casting|CastToBP_FirstPersonCharacter OtherActor))
      (CallFunction|OnInteract _asbp_first_person_character))))

(event OnComponentBeginOverlap(Sphere)
  (params (OverlappedComponent :type Primitive%20Component%20Object%20Reference) (OtherActor :type Actor%20Object%20Reference) (OtherComp :type Primitive%20Component%20Object%20Reference) (OtherBodyIndex :type Integer) (bFromSweep :type Boolean) (SweepResult :type Hit%20Result%20Structure%20%28by%20ref%29))
  ;[0.15 0.15 0.15 0.5] Interact Icon (Far)
  (if (== OtherActor (Game|GetPlayerCharacter 0))
    (Rendering|SetVisibility (Variables|Default|GetFarInteractIcon) true false)
    (Rendering|SetVisibility (Variables|Default|GetNearInteractIcon) false false)))

(event OnComponentEndOverlap(Sphere)
  (params (OverlappedComponent :type Primitive%20Component%20Object%20Reference) (OtherActor :type Actor%20Object%20Reference) (OtherComp :type Primitive%20Component%20Object%20Reference) (OtherBodyIndex :type Integer))
  ;[0.15 0.15 0.15 0.5] Interact Icon (Far)
  (if (== (Game|GetPlayerCharacter 0) OtherActor)
    (Rendering|SetVisibility (Variables|Default|GetFarInteractIcon) false false)
    (Rendering|SetVisibility (Variables|Default|GetNearInteractIcon) false false)))

(event Custom|HandleRotation
  (params (TargetRotation :type Float%20%28double-precision%29))
  ;[0.15 0.15 0.15 0.5] Handle Rotation
  (Transformation|SetRelativeRotation (Variables|Default|GetDoor) (Math|Rotator|MakeRotator 0.0 0.0 (Math|Interpolation|FInterpTo (.Yaw (Math|Rotator|BreakRotator (Variables|/Script/Engine.SceneComponent|GetRelativeRotation (Variables|Default|GetDoor)))) TargetRotation (Utilities|Time|GetWorldDeltaSeconds) (Variables|Door|GetRotationSpeed))) false false))

(event Custom|HandleDoor
  ;[0.15 0.15 0.15 0.5] Handle Door
  (switch Utilities|FlowControl|Switch|SwitchonE_DoorState (Variables|Default|GetCurrentDoorState)
    (:NewEnumerator0
      (CallFunction|HandleRotation (* (Variables|Default|GetCurrentDoorSide) (Variables|Door|GetPartialOpenRotation))))
    (:NewEnumerator1
      (CallFunction|HandleRotation (* (Variables|Default|GetCurrentDoorSide) (Variables|Door|GetCompletelyOpenRotation))))
    (:NewEnumerator2
      (CallFunction|HandleRotation 0.0))))

(event Custom|onInteract
  (params (Character :type BP%20First%20Person%20Character%20Object%20Reference))
  ;[0.15 0.15 0.15 0.5] Interact Logic
  (CallFunction|PlaySound)
  (if (> (Math|Vector|DotProduct (Transformation|GetActorForwardVector Character) (Math|Vector|GetForwardVector (Variables|Default|GetDoorLookPosition))) 0.0)
    (Variables|Default|SetCurrentDoorSide 1.0)
    (else
      (Variables|Default|SetCurrentDoorSide -1.0)))
  (Variables|Default|SetbIsInteracting true)
  (Utilities|Time|SetTimerbyEvent (delegate Custom|onStopInteract) (Variables|Default|GetDoorSoundTime)))

(event Custom|onStopInteract
  ;[0.15 0.15 0.15 0.5] Interact Logic
  (Variables|Default|SetbIsInteracting false)
  (switch Utilities|FlowControl|Switch|SwitchonE_DoorState (Variables|Default|GetCurrentDoorState)
    (:NewEnumerator0
      (Variables|Default|SetCurrentDoorState "NewEnumerator1"))
    (:NewEnumerator1
      (Variables|Default|SetCurrentDoorState "NewEnumerator2"))
    (:NewEnumerator2
      (Variables|Default|SetCurrentDoorState "NewEnumerator0"))))

(event Custom|PlaySound
  (bind _returnvalue (Transformation|GetActorLocation))
  ;[0.15 0.15 0.15 0.5] Sounds
  (switch Utilities|FlowControl|Switch|SwitchonE_DoorState (Variables|Default|GetCurrentDoorState)
    (:NewEnumerator0
      (Audio|PlaySoundatLocation "/Game/Audio/Door/DOOR_Wood_Bedroom_Open_02_mono.DOOR_Wood_Bedroom_Open_02_mono" _returnvalue "0, 0, 0" 1.0 1.0 0.0 0 0 0 0))
    (:NewEnumerator1
      (Audio|PlaySoundatLocation "/Game/Audio/Door/CREAK_Door_05_mono.CREAK_Door_05_mono" _returnvalue "0, 0, 0" 1.0 1.0 0.0 0 0 0 0))
    (:NewEnumerator2
      (Audio|PlaySoundatLocation "/Game/Audio/Door/DOOR_Apartment_Close_stereo.DOOR_Apartment_Close_stereo" _returnvalue "0, 0, 0" 1.0 1.0 0.0 0 0 0 0))))

(event EventBeginPlay
  (bind _asbp_first_person_character (Utilities|Casting|CastToBP_FirstPersonCharacter (Game|GetPlayerCharacter 0)))
  (Variables|Default|SetCharacterRef _asbp_first_person_character)
  (Rendering|SetVisibility (Variables|Default|GetNearInteractIcon) false false)
  (Rendering|SetVisibility (Variables|Default|GetFarInteractIcon) false false))

(event EventTick
  (params (DeltaSeconds :type Float%20%28single-precision%29))
  (if (Variables|Default|GetbIsInteracting)
    (CallFunction|HandleDoor)))

(event EventInteract
  (params (Interactor :type Character%20Object%20Reference))
  (bind _characterref (Variables|Default|GetCharacterRef))
  ;[0.15 0.15 0.15 0.5] Interactable Interface implementation
  (if (== (Variables|/Game/Blueprints/GameFramework/BP_FirstPersonCharacter.BP_FirstPersonCharacter_C|GetCurrentHitInteractable _characterref) self)
    (CallFunction|OnInteract _characterref)))

(event EventCanInteract
  (params (bCanInteract :type Boolean))
  ;[0.15 0.15 0.15 0.5] Interactable Interface implementation
  (Rendering|SetVisibility (Variables|Default|GetNearInteractIcon) bCanInteract false))

(fn ConstructionScript)